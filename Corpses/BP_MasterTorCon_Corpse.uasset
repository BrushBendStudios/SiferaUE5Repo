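; Base corpse actor that the player can search once through the SGK interaction interface.
; While CanBeSearched is true it allows interaction and offers a "Search" action, labelled with CorpseName.
; Interacting plays the BodySearchedDialogue 2D sound and clears the flag, granting no items.
; The other interface functions are empty or return defaults, and the event graph and construction script are unused.
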(event EventBeginPlay)

(event Collision|EventActorBeginOverlap
  (params (OtherActor :type Actor%20Object%20Reference)))

(event EventTick
  (params (DeltaSeconds :type Float%20%28single-precision%29)))

(fn ConstructionScript)

(fn SGKAllowInteraction
  (if (Variables|Default|GetCanBeSearched)
    (return true)
    (else
      (return false))))

(fn SGKCodeCheck
  (params (Code :type Text))
  (return false))

(fn SGKDropItem
  (params (InvItem :type S%20Inv%20Item%20Structure) (Dropped :type Boolean) (Spawned :type Boolean) (SaveLoaded :type Boolean))
  (return false))

(fn SGKEndHighlight
  (return false))

(fn SGKEndInteraction
  (params (PlayerInventory :type BP%20Player%20Inventory%20Object%20Reference))
  (return false))

(fn SGKGetVerifiedPlayers
  (return 0))

(fn SGKInteract
  (params (PlayerInventory :type BP%20Player%20Inventory%20Object%20Reference) (Action :type E_WorldActions%20Enum :default "NewEnumerator0"))
  (Audio|PlaySound2D (Variables|Default|GetBodySearchedDialogue) 1.0 1.0 0.0 0 0)
  (Variables|Default|SetCanBeSearched false)
  (return true))

(fn SGKInteractName
  (return (Variables|Default|GetCorpse%20name)))

(fn SGKInvItem
  (return false ""))

(fn SGKItemAmount
  (return 0))

(fn SGKMesh
  (return 0))

(fn SGKPossibleActions
  (params (PlayerInventory :type BP%20Player%20Inventory%20Object%20Reference) (PlayerCharacter :type BP%20SGK%20Master%20Character%20Object%20Reference))
  (if (Variables|Default|GetCanBeSearched)
    (return true (Utilities|Array|MakeArray (Utilities|Struct|MakeS_WorldAction "NewEnumerator8" "Search")))
    (else
      (return false 0))))

(fn SGKStartHighlight
  (return false))

(fn SGKUpdateCode
  (params (Code :type Text))
  (return false))

(fn SGKVerifyPlayer
  (params (Text :type Text))
  (return false))