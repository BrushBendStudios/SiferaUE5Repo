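; Mission terminal actor that players use through the SGK interaction interface to open the mission terminal UI.
; It offers a single "Use" action, with interaction allowed only while CanBeAccessed is true.
; Interact creates the terminal widget for the interacting player's HUD owner through a FlipFlop, so only every other call opens it.
; BeginPlay caches the player character; the other interface functions are empty stubs.
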(event EventBeginPlay
  (bind _asbp_sgkmaster_character (Utilities|Casting|CastToBP_SGKMasterCharacter (Game|GetPlayerCharacter 0)))
  (Variables|Default|SetPlayer%20Ref _asbp_sgkmaster_character))

(fn ConstructionScript)

(fn SGKAllowInteraction
  (if (Variables|Default|GetCan%20Be%20Accessed)
    (return true)
    (else
      (return false))))

(fn SGKCodeCheck
  (params (Code :type Text))
  (return false))

(fn SGKDropItem
  (params (InvItem :type S%20Inv%20Item%20Structure) (Dropped :type Boolean) (Spawned :type Boolean) (SaveLoaded :type Boolean))
  (return false))

(fn SGKEndHighlight
  (return false))

(fn SGKEndInteraction
  (params (PlayerInventory :type BP%20Player%20Inventory%20Object%20Reference))
  (return false))

(fn SGKGetVerifiedPlayers
  (return 0))

(fn SGKInteract
  (params (PlayerInventory :type BP%20Player%20Inventory%20Object%20Reference) (Action :type E_WorldActions%20Enum :default "NewEnumerator0"))
  (Utilities|FlowControl|FlipFlop
    (:A
      (bind _returnvalue (UserInterface|CreateWidget "/Game/_MissionSystem/BP_Mission_Terminal_Widget.BP_Mission_Terminal_Widget_C" (Widget|GetOwningPlayer (Variables|/Game/SurvivalGameKitV2/Blueprints/Components/BP_PlayerInventory.BP_PlayerInventory_C|GetPlayerHUD PlayerInventory))))
      (bind _output_get (Variables|Default|SetWidgetRef _returnvalue))
      (UserInterface|Viewport|AddtoViewport _output_get 505)
      (return true))))

(fn SGKInteractName
  (return ""))

(fn SGKInvItem
  (return false ""))

(fn SGKItemAmount
  (return 0))

(fn SGKMesh
  (return 0))

(fn SGKPossibleActions
  (params (PlayerInventory :type BP%20Player%20Inventory%20Object%20Reference) (PlayerCharacter :type BP%20SGK%20Master%20Character%20Object%20Reference))
  (return true (Utilities|Array|MakeArray (Utilities|Struct|MakeS_WorldAction "NewEnumerator8" "Use"))))

(fn SGKStartHighlight
  (return false))

(fn SGKUpdateCode
  (params (Code :type Text))
  (return false))

(fn SGKVerifyPlayer
  (params (Text :type Text))
  (return false))