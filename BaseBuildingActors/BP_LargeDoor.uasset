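; BP_LargeDoor is a base-building sliding door that opens only for SGK master characters with the "AlphaAccess" skill.
; Box overlap plays a hydraulic sound at world origin for any actor, then checks the skill before a timeline slides the mesh.
; When the timeline finishes, it waits five seconds, replays the sound and reverses.
; A separate OpenDoor event instead moves the whole actor to an offset from the mesh's location.
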(event OnComponentBeginOverlap(Box)
  (params (OverlappedComponent :type Primitive%20Component%20Object%20Reference) (OtherActor :type Actor%20Object%20Reference) (OtherComp :type Primitive%20Component%20Object%20Reference) (OtherBodyIndex :type Integer) (bFromSweep :type Boolean) (SweepResult :type Hit%20Result%20Structure%20%28by%20ref%29))
  (Audio|PlaySoundatLocation "/Game/_Sounds/PM_Foundation_Series_SCI-FI_vol_2/PM_FSSF2_DOOR_BIG_HYDRAULIC_4.PM_FSSF2_DOOR_BIG_HYDRAULIC_4" "0, 0, 0" "0, 0, 0" 0.75 0.95 0.0 0 0 0 0)
  (bind _asbp_sgkmaster_character (Utilities|Casting|CastToBP_SGKMasterCharacter OtherActor))
  (bind _success (Default|QuerySkill (Variables|/Game/SurvivalGameKitV2/Blueprints/Characters/BP_SGKMasterCharacter.BP_SGKMasterCharacter_C|GetSkillSystemComponent _asbp_sgkmaster_character) "AlphaAccess"))
  (if _success
    (bind _slide (Timeline|SlidingDoorAnim Play)
      (:Update
        (Transformation|SetRelativeLocation (Variables|Default|GetStaticMesh) _slide false false))
      (:Finished
        (Utilities|FlowControl|Delay 5.0)
        (Audio|PlaySoundatLocation "/Game/_Sounds/PM_Foundation_Series_SCI-FI_vol_2/PM_FSSF2_DOOR_BIG_HYDRAULIC_4.PM_FSSF2_DOOR_BIG_HYDRAULIC_4" "0, 0, 0" "0, 0, 0" 0.75 0.95 0.0 0 0 0 0)
        (Timeline|SlidingDoorAnim Reverse)))))

(event OnComponentEndOverlap(Box)
  (params (OverlappedComponent :type Primitive%20Component%20Object%20Reference) (OtherActor :type Actor%20Object%20Reference) (OtherComp :type Primitive%20Component%20Object%20Reference) (OtherBodyIndex :type Integer)))

(event Custom|OpenDoor
  (Transformation|SetActorLocation (- (Transformation|GetWorldLocation (Variables|Default|GetStaticMesh)) "0,-120.000000, 0") true false))

(fn ConstructionScript)