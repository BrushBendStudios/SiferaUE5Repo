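; Interactable base-building Armor Terminal that gives the player access to the character selection screen.
; Implements the SGK interaction functions, offering a single "Use" action that calls ToggleCharacterSelect on the interacting player's HUD; the other functions are stubs.
; BeginPlay also creates a BP_CharacterSelect widget for player controller 0 and stores it, but the interaction does not use that reference.
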(event EventBeginPlay
  (bind _returnvalue (UserInterface|CreateWidget "/Game/BP_CharacterSelect.BP_CharacterSelect_C" (Game|GetPlayerController 0)))
  (Variables|Default|SetCharacterSelectionRef _returnvalue))

(fn ConstructionScript)

(fn SGKAllowInteraction
  (return true))

(fn SGKCodeCheck
  (params (Code :type Text))
  (return false))

(fn SGKDropItem
  (params (InvItem :type S%20Inv%20Item%20Structure) (Dropped :type Boolean) (Spawned :type Boolean) (SaveLoaded :type Boolean))
  (return false))

(fn SGKEndHighlight
  (return false))

(fn SGKEndInteraction
  (params (PlayerInventory :type BP%20Player%20Inventory%20Object%20Reference))
  (return false))

(fn SGKGetVerifiedPlayers
  (return 0))

(fn SGKInteract
  (params (PlayerInventory :type BP%20Player%20Inventory%20Object%20Reference) (Action :type E_WorldActions%20Enum :default "NewEnumerator0"))
  (Default|ToggleCharacterSelect (Variables|/Game/SurvivalGameKitV2/Blueprints/Components/BP_PlayerInventory.BP_PlayerInventory_C|GetPlayerHUD PlayerInventory))
  (return false))

(fn SGKInteractName
  (return "Armor Terminal"))

(fn SGKInvItem
  (return false ""))

(fn SGKItemAmount
  (return 0))

(fn SGKMesh
  (return 0))

(fn SGKPossibleActions
  (params (PlayerInventory :type BP%20Player%20Inventory%20Object%20Reference) (PlayerCharacter :type BP%20SGK%20Master%20Character%20Object%20Reference))
  (return true (Utilities|Array|MakeArray (Utilities|Struct|MakeS_WorldAction "NewEnumerator8" "Use"))))

(fn SGKStartHighlight
  (return false))

(fn SGKUpdateCode
  (params (Code :type Text))
  (return false))

(fn SGKVerifyPlayer
  (params (Text :type Text))
  (return false))